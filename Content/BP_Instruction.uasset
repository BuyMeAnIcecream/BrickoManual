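; BP_Instruction is an actor that plays a step-by-step assembly of static mesh parts, one piece per NextPiece call.
; BeginPlay gathers child meshes into Parts, while InitPieces lists named parts and highlight meshes.
; Each step, locked during movement, scales the piece's relative location by a timeline, then reveals the next part and hides the placed part's highlight.
; A separate event plays a blue dissolve before restoring cached materials.
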(event Custom|ProcessPiecePlacement
  (params (PieceMesh :type Static%20Mesh%20Component%20Object%20Reference))
  (Variables|Default|SetInitLoc (Variables|/Script/Engine.SceneComponent|GetRelativeLocation PieceMesh))
  (bind _progression (Timeline|Timeline_0 PlayFromStart)
    (:Update
      (Transformation|SetRelativeLocation PieceMesh (* _progression (Variables|Default|GetInitLoc)) false false))
    (:Finished
      (Variables|Default|SetInMovement false)
      (Development|SetHiddeninGame (Utilities|Array|Get(acopy) (Variables|Default|GetParts) (Variables|Default|GetPieceIdx)) false true)
      (Development|SetHiddeninGame (Utilities|Array|Get(acopy) (Variables|Default|GetPartsHighlight) (- (Variables|Default|GetPieceIdx) 1)) true true))))

(event Custom|NextPiece
  (bind _pieceidx (Variables|Default|GetPieceIdx))
  (bind _parts (Variables|Default|GetParts))
  (bind _output (Utilities|Array|Get(acopy) _parts _pieceidx))
  (Utilities|IsValid _output
    (:Is%20Valid
      (if (not (Variables|Default|GetInMovement))
        (Variables|Default|SetInMovement true)
        (CallFunction|ProcessPiecePlacement _output)
        (Math|Integer|IncrementInt (Variables|Default|GetPieceIdx))))))

(event Custom|CustomEvent_0
  (bind _output_get (Variables|Default|SetCachedMaterials (Rendering|Material|GetMaterials (stale Custom|ProcessPiecePlacement PieceMesh))))
  (for (_ _array_index) _output_get
    (bind _returnvalue (Rendering|Material|CreateDynamicMaterialInstance "/Game/Materials/MI_DissolveBlue.MI_DissolveBlue" "None" "None" :!class /Script/Engine.KismetMaterialLibrary))
    (Rendering|Material|SetMaterial (stale Custom|ProcessPiecePlacement PieceMesh) _array_index _returnvalue)
    (bind _newtrack_0 (Timeline|Timeline_1 PlayFromStart)
      (:Update
        (Rendering|Material|SetScalarParameterValue _returnvalue "Dissolve" _newtrack_0 :!class /Script/Engine.MaterialInstanceDynamic))
      (:Finished
        (Rendering|Material|SetMaterial (stale Custom|ProcessPiecePlacement PieceMesh) _array_index (Utilities|Array|Get(acopy) (Variables|Default|GetCachedMaterials) _array_index))))))

(event EventBeginPlay
  (for _array_element (Components|GetChildrenComponents (Variables|Default|GetDefaultSceneRoot) false)
    (bind _asstatic_mesh_component (Utilities|Casting|CastToStaticMeshComponent _array_element))
    (Utilities|Array|Add (Variables|Default|GetParts) _asstatic_mesh_component)))

(fn ConstructionScript)

(fn InitPieces
  (bind _parts (Variables|Default|GetParts))
  (bind _parts_2 (Variables|Default|GetParts))
  (bind _parts_3 (Variables|Default|GetParts))
  (bind _parts_4 (Variables|Default|GetParts))
  (Utilities|FlowControl|Sequence
    (:then_0
      (Utilities|Array|Add (Variables|Default|GetParts) (Variables|Default|GetBlueCabinBase))
      (Utilities|Array|Add _parts_4 (Variables|Default|GetHood1))
      (Utilities|Array|Add _parts_4 (Variables|Default|GetHood2))
      (Utilities|Array|Add _parts_2 (Variables|Default|GetHood3))
      (Utilities|Array|Add _parts_2 (Variables|Default|GetStaticMesh2))
      (Utilities|Array|Add _parts_2 (Variables|Default|GetStaticMesh3))
      (Utilities|Array|Add _parts_2 (Variables|Default|GetStaticMesh4))
      (Utilities|Array|Add _parts (Variables|Default|GetTrunkBase))
      (Utilities|Array|Add _parts (Variables|Default|GetFlower1))
      (Utilities|Array|Add _parts_3 (Variables|Default|GetFlower2))
      (Utilities|Array|Add _parts_3 (Variables|Default|GetFlower4))
      (Utilities|Array|Add _parts_3 (Variables|Default|GetFlower3))
      (Utilities|Array|Add _parts_3 (Variables|Default|GetBunny)))
    (:then_1
      (Utilities|Array|Add (Variables|Default|GetPartsHighlight) (Variables|Default|GetBlueCabinBase_Highlight))
      (Utilities|Array|Add (Variables|Default|GetPartsHighlight) (Variables|Default|GetHood1_Highlight))
      (Utilities|Array|Add (Variables|Default|GetPartsHighlight) (Variables|Default|GetHood2_Highlight))
      (Utilities|Array|Add (Variables|Default|GetPartsHighlight) (Variables|Default|GetHood3_Highlight)))))